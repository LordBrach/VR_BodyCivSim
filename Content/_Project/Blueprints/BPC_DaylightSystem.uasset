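; Actor component that runs a day/night cycle and checks whether the level's lamp state matches it, on by day and off by night.
; Tick flips the phase after the day or night length and broadcasts the change with lamp correctness.
; A mismatch lasting beyond SafeTime fires a repeating daylight error event.
; It finds a BP_Lamp if none is set and rebroadcasts its switches as correct or incorrect.
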(event Custom|OnLightSwitched
  (params (IsOn :type Boolean))
  (bind _isday (Variables|Default|GetIsDay))
  (Default|CallOnLampSwitched (== IsOn _isday) _isday))

(event EventTick
  (params (DeltaSeconds :type Float%20%28single-precision%29))
  (Utilities|FlowControl|Sequence
    (:then_0
      (bind _output_get (Variables|Default|SetDayTime (+ (Variables|Default|GetDayTime) DeltaSeconds)))
      (if (> _output_get (Math|Float|SelectFloat (Variables|Default|GetDayLength) (Variables|Default|GetNightLength) (Variables|Default|GetIsDay)))
        (bind _output_get_2 (Variables|Default|SetIsDay (not (Variables|Default|GetIsDay))))
        (Default|CallOnDayChanged _output_get_2 (== _output_get_2 (Variables|/Game/_Project/Blueprints/InteractableObjects/BP_Lamp.BP_Lamp_C|GetIsOn (Variables|Default|GetLamp))))
        (Variables|Default|SetDayTime 0.0)))
    (:then_1
      (if (!= (Variables|Default|GetIsDay) (Variables|/Game/_Project/Blueprints/InteractableObjects/BP_Lamp.BP_Lamp_C|GetIsOn (Variables|Default|GetLamp)))
        (bind _output_get_3 (Variables|Default|SetErrorTime (+ (Variables|Default|GetErrorTime) DeltaSeconds)))
        (if (> _output_get_3 (Variables|Default|GetSafeTime))
          (Default|CallOnDaylightError)
          (Variables|Default|SetErrorTime 0.0))
        (elif (> (Variables|Default|GetErrorTime) 0.01)
          (Variables|Default|SetErrorTime 0.0))))))

(event EventBeginPlay
  (Utilities|IsValid (Variables|Default|GetLamp)
    (:Is%20Valid
      _)
    (:Is%20Not%20Valid
      (bind _returnvalue (Actor|GetActorOfClass "/Game/_Project/Blueprints/InteractableObjects/BP_Lamp.BP_Lamp_C"))
      (bind _output_get (Variables|Default|SetLamp _returnvalue))))
  (Components|Tick|SetComponentTickEnabled (Utilities|IsValid _output_get))
  (EventDispatchers|BindEventtoOnLightSwitched _output_get (delegate Custom|OnLightSwitched)))
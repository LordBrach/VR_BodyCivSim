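; Game clock component that drives difficulty progression and timed in-game events through the DataJeuDuBidou game instance.
; Each tick, MainClock accumulates elapsed time during one game state and passes it to the game instance's event curve update.
; EventClock counts independently of that state; on reaching its target, it resets, takes the current difficulty value as the next interval, and fires in-game and random event calls.
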(event EventBeginPlay
  (bind _asdata_jeu_du_bidou (Utilities|Casting|CastToDataJeuDuBidou (Game|GetGameInstance)))
  (Variables|Default|SetData%20Jeu%20Du%20Bidou _asdata_jeu_du_bidou))

(event EventTick
  (params (DeltaSeconds :type Float%20%28single-precision%29))
  (CallFunction|MainClock DeltaSeconds)
  (CallFunction|EventClock DeltaSeconds))

(fn MainClock
  (params (InputPin :type Float%20%28single-precision%29))
  (if (Utilities|Enum|Equal(Enum) (Variables|/Game/_Project/Data/DataJeuDuBidou.DataJeuDuBidou_C|GetGameState (Variables|Default|GetData%20Jeu%20Du%20Bidou)) "NewEnumerator2")
    (bind _output_get (Variables|Default|SetTimer%20Val (+ InputPin (Variables|Default|GetTimer%20Val))))
    (bind _difficultyval (Default|UpdateEventCurve (Variables|Default|GetData%20Jeu%20Du%20Bidou) _output_get))))

(fn EventClock
  (params (Delta :type Float%20%28double-precision%29))
  (Variables|Default|SetEventTimer (+ (Variables|Default|GetEventTimer) Delta))
  (if (>= (Variables|Default|GetEventTimer) (Variables|Default|GetEventTimerTarget))
    (Variables|Default|SetEventTimer 0.0)
    (Variables|Default|SetEventTimerTarget (Variables|/Game/_Project/Data/DataJeuDuBidou.DataJeuDuBidou_C|GetCurrentDifficultyVal (Variables|Default|GetData%20Jeu%20Du%20Bidou)))
    (Default|CallInGameEvent)
    (Default|CallCallRandomEvent (Variables|Default|GetData%20Jeu%20Du%20Bidou))
    (Development|PrintText (Utilities|Text|FormatText "Start in game event here, after {target} seconds of waiting" 0))))
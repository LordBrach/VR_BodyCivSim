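; BP_Body is the central "Bidou" body actor, whose attached tummy houses act as its health: losing the last one ends the game.
; On game start it spawns DefaultHP houses at shuffled child-actor spawn points.
; It ticks water, daylight and hunger components from a game clock, and their failure events destroy random houses, with tsunamis also firing a geyser there.
; State changes drive warning popups, sounds and house window lighting.
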(event OnDroughtTriggered(BPC_WaterComponent)
  ;[0.15 0.15 0.15 0.5] ReceiveEvents
  (CallFunction|DestroyRandomHouse))

(event OnDaylightError(BPC_DaylightSystem)
  ;[0.15 0.15 0.15 0.5] ReceiveEvents
  (CallFunction|DestroyRandomHouse))

(event OnLampSwitched(BPC_DaylightSystem)
  (params (IsCorrect :type Boolean) (IsDay :type Boolean))
  ;[0.15 0.15 0.15 0.5] Event state change
  (CallFunction|OnPopUpUpdate IsCorrect IsDay))

(event OnTsunamiTriggered(BPC_WaterComponent)
  (bind _geyser (Variables|Default|GetGeyser))
  ;[0.15 0.15 0.15 0.5] ReceiveEvents
  (Default|PlaySoundSpatialized (Variables|Default|GetBPC_SoundPlayer) "Tsunami")
  (bind _housetransform (CallFunction|DestroyRandomHouse))
  (Transformation|SetWorldLocationAndRotation _geyser (.location _housetransform) (.rotation _housetransform) false true)
  (Components|Activation|Activate _geyser true)
  (Utilities|FlowControl|Delay (Variables|Animation|GetGeyserDuration))
  (Components|Activation|Deactivate (Variables|Default|GetGeyser)))

(event OnWaterStateChanged(BPC_WaterComponent)
  (params (WaterState :type EN_WaterState%20Enum :default "NewEnumerator4"))
  (bind _popupmanager (Variables|Default|GetPopupManager))
  ;[0.15 0.15 0.15 0.5] Event state change
  (Utilities|IsValid _popupmanager
    (:Is%20Valid
      (switch Utilities|FlowControl|Switch|SwitchonEN_WaterState WaterState
        (:NewEnumerator4
          (Default|RemovePopup _popupmanager "NewEnumerator4")
          (Default|RemovePopup _popupmanager "NewEnumerator3"))
        (:NewEnumerator1
          (Default|AddPopup _popupmanager "NewEnumerator4"))
        (:NewEnumerator2
          (Default|AddPopup _popupmanager "NewEnumerator3"))))))

(event OnStarveLaunched(BPC_HungerSystem)
  ;[0.15 0.15 0.15 0.5] ReceiveEvents
  (CallFunction|DestroyRandomHouse))

(event OnStateChanged(BPC_HungerSystem)
  (params (New%20State :type EN_HungerState%20Enum :default "NewEnumerator0"))
  (bind _popupmanager (Variables|Default|GetPopupManager))
  ;[0.15 0.15 0.15 0.5] Event state change
  (if (Utilities|Enum|Equal(Enum) New%20State "NewEnumerator0")
    (Default|RemovePopup _popupmanager "NewEnumerator5")
    (else
      (Default|AddPopup _popupmanager "NewEnumerator5")
      (Default|PlaySoundSpatialized (Variables|Default|GetBPC_SoundPlayer) "Gargouillement"))))

(event OnDayChanged(BPC_DaylightSystem)
  (params (IsDay :type Boolean) (IsLampCorrect :type Boolean))
  ;[0.15 0.15 0.15 0.5] Event state change
  (CallFunction|OnPopUpUpdate IsLampCorrect IsDay)
  (CallFunction|UpdateHousesDay IsDay false))

(event Custom|SetupBidou
  ;[0.15 0.15 0.15 0.5] BeginPlay
  (CallFunction|UpdateSpawnPoints)
  (CallFunction|SpawnHouses)
  (CallFunction|UpdateHousesDay (Variables|/Game/_Project/Blueprints/BPC_DaylightSystem.BPC_DaylightSystem_C|GetIsDay (Variables|Default|GetBPC_DaylightSystem)) true))

(event Custom|ReceiveHouseDestroyed
  (params (HouseToDestroy :type BP%20Tummy%20House%20Object%20Reference))
  ;[0.15 0.15 0.15 0.5] HouseDestroyed
  (bind _returnvalue (Utilities|Array|RemoveItem (Variables|Default|GetHouses) HouseToDestroy))
  (if _returnvalue
    (Development|PrintText "Deleted a house" true true "(R=0.082822,G=1.000000,B=0.000000,A=1.000000)")
    (if (Utilities|Array|IsEmpty (Variables|Default|GetHouses))
      (Default|EndGame (Variables|Default|GetData%20Jeu%20Du%20Bidou)))
    (else
      (Development|PrintText "Couldnt Delete house" true true "(R=1.000000,G=0.000000,B=0.000000,A=1.000000)"))))

(event Custom|EatFood
  (params (FoodValue :type Float%20%28double-precision%29))
  ;[0.15 0.15 0.15 0.5] EAT/DRINK
  (Default|AddFood (Variables|Default|GetBPC_HungerSystem) FoodValue))

(event Custom|OnPopUpUpdate
  (params (IsCorrect :type Boolean) (IsDay :type Boolean))
  (bind _popupmanager (Variables|Default|GetPopupManager))
  ;[0.15 0.15 0.15 0.5] Event state change
  (if IsCorrect
    (Default|RemovePopup _popupmanager "NewEnumerator6")
    (Default|RemovePopup _popupmanager "NewEnumerator7")
    (else
      (Default|AddPopup _popupmanager (select IsDay "NewEnumerator6" "NewEnumerator7")))))

(event EventBeginPlay
  ;[0.15 0.15 0.15 0.5] BeginPlay
  (bind _asdata_jeu_du_bidou (Utilities|Casting|CastToDataJeuDuBidou (Game|GetGameInstance)))
  (bind _output_get (Variables|Default|SetData%20Jeu%20Du%20Bidou _asdata_jeu_du_bidou))
  (Variables|/Game/_Project/Data/DataJeuDuBidou.DataJeuDuBidou_C|SetBody _asdata_jeu_du_bidou self)
  (EventDispatchers|BindEventtoEventStartGame _output_get (delegate Custom|SetupBidou))
  (if (Variables|Default|GetAutoStartGame)
    ;;[0.15 0.15 0.15 0.5] StartGame
    (Default|StartGame _output_get)))

(event EventAddWater
  (params (DeltaTime :type Float%20%28double-precision%29))
  ;[0.15 0.15 0.15 0.5] EAT/DRINK
  (Default|AddWater (Variables|Default|GetBPC_WaterComponent) DeltaTime))

(event EventTick
  (params (DeltaSeconds :type Float%20%28single-precision%29))
  (bind _bpc_gameclock (Variables|Default|GetBPC_GameClock))
  (bind _timer_val (Variables|/Game/_Project/Blueprints/Gameloop/BPC_GameClock.BPC_GameClock_C|GetTimer%20Val _bpc_gameclock))
  ;[0.15 0.15 0.15 0.5] TICK
  (Default|Update (Variables|Default|GetBPC_WaterComponent) DeltaSeconds _timer_val)
  (Default|Update (Variables|Default|GetBPC_DaylightSystem) DeltaSeconds _timer_val)
  (Default|Update (Variables|Default|GetBPC_HungerSystem) DeltaSeconds _timer_val)
  (Default|CETick (Variables|Default|GetBPC_GameClock) DeltaSeconds))

(fn ConstructionScript)

(fn SpawnHouses
  (bind _spawnpoints (Variables|Default|GetSpawnPoints))
  (Utilities|Array|Shuffle _spawnpoints)
  (bind (_array_element _array_index) (Utilities|Array|ForEachLoopwithBreak _spawnpoints)
    (:LoopBody
      (if (< _array_index (Variables|/Game/_Project/Data/DataJeuDuBidou.DataJeuDuBidou_C|GetDefaultHP (Variables|Default|GetData%20Jeu%20Du%20Bidou)))
        (bind _asbp_house_spawn_location (Utilities|Casting|CastToBP_HouseSpawnLocation (Variables|/Script/Engine.ChildActorComponent|GetChildActor _array_element))
          (:then
            (bind _returnvalue (Game|SpawnActorfromClass "/Game/_Project/Blueprints/Gameloop/BP_TummyHouse.BP_TummyHouse_C" (Transformation|GetActorTransform _asbp_house_spawn_location) "Undefined" "MultiplyWithRoot" 0 0))
            (bind _output_get (Variables|/Game/_Project/Blueprints/Gameloop/BP_HouseSpawnLocation.BP_HouseSpawnLocation_C|SetLinkedHouse _asbp_house_spawn_location _returnvalue))
            (Transformation|AttachActorToActor _returnvalue self "None" "KeepWorld" "KeepWorld" "KeepWorld" true)
            (Variables|/Game/_Project/Blueprints/Gameloop/BP_TummyHouse.BP_TummyHouse_C|SetOwnerBody _output_get self)
            (Utilities|Array|Add (Variables|Default|GetHouses) _output_get))
          (:CastFailed
            (Development|PrintText "Couldnt cast to bp_house")
            (return)))))
    (:Completed
      (return))))

(fn UpdateSpawnPoints
  (Utilities|Array|Clear (Variables|Default|GetSpawnPoints))
  (for _array_element (Components|GetChildrenComponents (Variables|Default|GetBodyMesh) false)
    (bind _aschild_actor_component (Utilities|Casting|CastToChildActorComponent _array_element))
    (Utilities|Array|Add (Variables|Default|GetSpawnPoints) _aschild_actor_component)))

(fn UpdateHousesDay
  (params (IsDay :type Boolean) (SkipDelay :type Boolean))
  (for _array_element (Variables|Default|GetHouses)
    (Default|UpdateWindows _array_element IsDay SkipDelay)))

(fn DestroyRandomHouse
  (bind _houses (Variables|Default|GetHouses))
  (if (Utilities|Array|IsNotEmpty _houses)
    (bind _output_get (LocalVariables|SetHouse (.OutItem (Utilities|Array|Random _houses))))
    (Default|DestroyHouse _output_get)
    (return (Transformation|GetActorTransform _output_get))))
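; Small animated NPC that walks along an assigned spline, or stands happy without one, and reacts through Walk, Happy, Panic and Die states.
; Tick advances spline distance and rolls timed random events; Direction toggles, but movement only goes forward.
; State changes feed ABP_PionAnims and sounds, with emotion changes randomly delayed to stagger reactions.
; Death plays a sound, then destroys the actor when audio finishes.
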(event Custom|OnDie
  ;[0.15 0.15 0.15 0.5] Death
  (Variables|Default|SetPionState "NewEnumerator1")
  (CallFunction|PlayAnim)
  (CallFunction|CEPlaySoundDeath)
  (EventDispatchers|BindEventtoOnAudioFinished (Variables|Default|GetAudio) (delegate Custom|DestroySelf)))

(event Custom|OnBirth
  ;[0.15 0.15 0.15 0.5] Spawn
  (CallFunction|SetupAnimBlueprint)
  (Variables|Default|GetSplineRef
    (:then
      (Variables|Default|SetCanMove true)
      (Variables|Default|SetPionState "NewEnumerator0"))
    (:else
      (Variables|Default|SetCanMove false)
      (Variables|Default|SetPionState "NewEnumerator2")))
  (CallFunction|PlayAnim))

(event Custom|CE_PlaySoundHappy
  ;[0.15 0.15 0.15 0.5] PlaySound
  (CallFunction|PlaySound "NewEnumerator2"))

(event Custom|CE_PlaySoundDeath
  ;[0.15 0.15 0.15 0.5] PlaySound
  (CallFunction|PlaySound "NewEnumerator1"))

(event Custom|CE_PlaySoundFear
  ;[0.15 0.15 0.15 0.5] PlaySound
  (CallFunction|PlaySound "NewEnumerator3"))

(event Custom|DestroySelf
  ;[0.15 0.15 0.15 0.5] Death
  (Utilities|FlowControl|Delay 0.2)
  (Actor|DestroyActor))

(event Custom|ChangeEmotion
  (params (InEmotion :type BPE_PionStates%20Enum :default "NewEnumerator0"))
  ;[0.15 0.15 0.15 0.5] Change Emotion
  (Variables|Default|SetPionState InEmotion)
  (Utilities|FlowControl|Delay (Math|Random|RandomFloatinRange 0.0 2.0))
  (CallFunction|PlaySoundEmotion)
  (CallFunction|PlayAnim))

(event EventTick
  (params (DeltaSeconds :type Float%20%28single-precision%29))
  ;[0.15 0.15 0.15 0.5] Main Loop
  (if (Variables|Default|GetCanMove)
    (CallFunction|UpdateSplineVal DeltaSeconds)
    (CallFunction|UpdatePosition)
    (CallFunction|RandomEvents DeltaSeconds)))

(fn ConstructionScript)

(fn UpdateSplineVal
  (params (InVal :type Float%20%28single-precision%29))
  (if true
    (Variables|Default|SetSplineVal (+ (Variables|Default|GetSplineVal) InVal))
    (else
      (Variables|Default|SetSplineVal (- (Variables|Default|GetSplineVal) InVal))))
  (return))

(fn UpdatePosition
  (bind _splineref (Variables|Default|GetSplineRef)
    (:then
      (Transformation|SetWorldLocation (Variables|Default|GetDefaultSceneRoot) (Spline|GetLocationatDistanceAlongSpline _splineref (Variables|Default|GetSplineVal) "World") false false))
    (:else
      (Variables|Default|SetCanMove false))))

(fn RandomEvents
  (params (InTime :type Float%20%28double-precision%29))
  (Variables|Default|SetTimer (+ (Variables|Default|GetTimer) InTime))
  (if (>= (Variables|Default|GetTimer) (LocalVariables|GetTimeTresholdRandom))
    (if (>= (Math|Random|RandomFloat) (LocalVariables|GetPercentage%20Chance))
      (Utilities|FlowControl|MultiGate true false -1
        (:Out%200
          (Variables|Default|SetPionState "NewEnumerator0")
          (CallFunction|PlayAnim)
          (Variables|Default|SetDirection (not (Variables|Default|GetDirection))))
        (:Out%201
          (CallFunction|PlaySoundEmotion)))
      (Variables|Default|SetTimer 0.0)
      (return))))

(fn PlaySoundEmotion
  (bind _bpc_soundplayer (Variables|Default|GetBPC_SoundPlayer))
  (switch Utilities|FlowControl|Switch|SwitchonBPE_PionStates (Variables|Default|GetPionState)
    (:NewEnumerator1
      (Default|PlaySoundSpatialized _bpc_soundplayer "PnjDead"))
    (:NewEnumerator2
      (Default|PlaySoundSpatialized _bpc_soundplayer "PnjHappy"))
    (:NewEnumerator3
      (Default|PlaySoundSpatialized _bpc_soundplayer "PnjScream"))))

(fn PlaySound
  (params (PionState :type BPE_PionStates%20Enum :default "NewEnumerator0"))
  (bind _audio (Variables|Default|GetAudio))
  (switch Utilities|FlowControl|Switch|SwitchonBPE_PionStates PionState
    (:NewEnumerator1
      (bind _out_sound (CallFunction|GetRandomSound (Variables|Default|GetSoundsFear)))
      (Audio|Components|Audio|SetSound _audio _out_sound))
    (:NewEnumerator2
      (bind _out_sound_2 (CallFunction|GetRandomSound (Variables|Default|GetSoundsHappy)))
      (Audio|Components|Audio|SetSound _audio _out_sound_2))
    (:NewEnumerator3
      (bind _out_sound_3 (CallFunction|GetRandomSound (Variables|Default|GetSoundsDeath)))
      (Audio|Components|Audio|SetSound _audio _out_sound_3)))
  (Audio|Components|Audio|Play _audio 0.0)
  (return))

(fn GetRandomSound
  (params (AudioArray :type Array%20of%20Sound%20Base%20Object%20References))
  (return (.OutItem (Utilities|Array|Random AudioArray))))

(fn SetupAnimBlueprint
  (bind _asabp_pion_anims (Utilities|Casting|CastToABP_PionAnims (Components|SkeletalMesh|GetAnimInstance (Variables|Default|GetSkeletalMesh)))
    (:then
      (bind _output_get (Variables|Default|SetABP_PionAnimsRef _asabp_pion_anims))
      (Default|ReceiveDataAnim _output_get "NewEnumerator0"))
    (:CastFailed
      (Development|PrintString "Cannot cast to ABP_PionANims"))))

(fn PlayAnim
  (bind _abp_pionanimsref (Variables|Default|GetABP_PionAnimsRef)
    (:then
      (Default|ReceiveDataAnim _abp_pionanimsref (Variables|Default|GetPionState)))
    (:else)))
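; VR-smashable house that spawns random inhabitants (BP_LilGuy) on a spline and picks one of two meshes.
; A fast motion-controller overlap or the death of its last inhabitant triggers destruction, with haptic feedback on smashes.
; Destruction kills all inhabitants, flings the mesh along a randomized timeline lerp with trail, explosion and sound, then notifies OwnerBody.
; Day/night updates recolor window lights, optionally after a random delay to stagger houses.
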(event Custom|HabitantDies
  (bind _habitantslist (Variables|Default|GetHabitantsList))
  (bind (_outitem _outindex) (Utilities|Array|Random _habitantslist))
  ;[0.15 0.15 0.15 0.5] KillHabitant
  (bind _result (Math|Integer|DecrementInt (Variables|Default|GetNbHabitants))
    (:%20%20
      (Default|OnDie _outitem)
      (Utilities|Array|RemoveIndex (Variables|Default|GetHabitantsList) _outindex)
      (if (== _result 0)
        (CallFunction|DestroyHouse)))))

(event Custom|DestroyHouse
  (bind _staticmesh (Variables|Default|GetStaticMesh))
  (bind _explosion (Variables|Default|GetExplosion))
  (bind _staticmesh_2 (Variables|Default|GetStaticMesh))
  (bind _deathrotationrange (Variables|Animation|GetDeathRotationRange))
  (bind _deathuprange (Variables|Animation|GetDeathUpRange))
  (bind _deathsiderange (Variables|Animation|GetDeathSideRange))
  (bind _returnvalue (Math|Random|RandomFloatinRange (.x _deathrotationrange) (.y _deathrotationrange)))
  (bind _returnvalue_2 (Math|Random|RandomFloatinRange (.x _deathsiderange) (.y _deathsiderange)))
  ;[0.15 0.15 0.15 0.5] Destroy House
  (Components|Activation|Activate (Variables|Default|GetTrail) true)
  (CallFunction|KillAllHabitants)
  (Utilities|FlowControl|DoOnce false
    (:Completed
      (bind _output_get (Variables|Animation|SetOriginDeathTransform (Transformation|GetWorldTransform _staticmesh_2)))
      (Variables|Animation|SetTargetDeathTransform (Math|Transform|MakeTransform (+ (.location _output_get) (* (Math|Vector|GetUpVector _staticmesh_2) (Math|Random|RandomFloatinRange (.x _deathuprange) (.y _deathuprange))) (* (Math|Vector|GetForwardVector _staticmesh_2) _returnvalue_2) (* (Math|Vector|GetRightVector _staticmesh_2) _returnvalue_2)) (Math|Rotator|CombineRotators (.rotation _output_get) (Math|Rotator|MakeRotator _returnvalue _returnvalue _returnvalue)) (.scale _output_get)))
      (bind (_direction _locationlerp _rotationlerp) (Timeline|DestroyAnimation PlayFromStart)
        (:Update
          (Transformation|SetWorldLocationAndRotation (Variables|Default|GetStaticMesh) (Math|Vector|Lerp(Vector) (.location (Variables|Animation|GetOriginDeathTransform)) (.location (Variables|Animation|GetTargetDeathTransform)) _locationlerp) (Math|Rotator|Lerp(Rotator) (.rotation (Variables|Animation|GetOriginDeathTransform)) (.rotation (Variables|Animation|GetTargetDeathTransform)) _rotationlerp true) false false))
        (:Finished
          (Default|ReceiveHouseDestroyed (Variables|Default|GetOwnerBody) self)
          (Default|CallOnHouseDestroyed)
          (Actor|DestroyActor))
        (:DestructionEvent
          (Development|SetHiddeninGame (Variables|Default|GetStaticMesh) true true)
          (Development|SetHiddeninGame _staticmesh true true)
          (Transformation|SetWorldLocationAndRotation _explosion (Transformation|GetWorldLocation _staticmesh) (Transformation|GetWorldRotation _staticmesh) false true)
          (Components|Activation|Activate _explosion true)
          (Default|PlaySoundSpatialized (Variables|Default|GetBPC_SoundPlayer) "HouseDestroy"))))))

(event Custom|UpdateWindows
  (params (IsDay :type Boolean) (SkipDelay :type Boolean))
  ;[0.15 0.15 0.15 0.5] Windows DayNight Update
  (if SkipDelay
    _
    (else
      (Utilities|FlowControl|Delay (Math|Random|RandomFloatinRange (Variables|Animation|GetWindowMinTime) (Variables|Animation|GetWindowMaxTime)))))
  (Rendering|Material|SetColorParameterValueonMaterials (Variables|Default|GetStaticMesh) "WindowLight" (Math|Color|SelectColor "(R=0.791298,G=0.644480,B=0.000000,A=1.000000)" "(R=0.011458,G=0.009308,B=0.000000,A=1.000000)" IsDay)))

(event EventBeginOverlap
  (params (MotionController :type Motion%20Controller%20Component%20Object%20Reference))
  ;[0.15 0.15 0.15 0.5] Hand Overlap
  (Variables|Default|SetMotion%20Controller MotionController)
  (if (> (Math|Vector|VectorLength (.OutLinearVelocity (Class|MotionControllerComponent|GetLinearVelocity (Variables|Default|GetMotion%20Controller)))) (Variables|Default|Getf_ImpulseForce))
    (CallFunction|DestroyHouse)
    (CallFunction|CEBeginOverlapFB)))

(event EventBeginPlay
  ;[0.15 0.15 0.15 0.5] Spawn Habitants
  (Components|StaticMesh|SetStaticMesh (Variables|Default|GetStaticMesh) (select (Math|Random|RandomBool) "/Game/_Project/Art/Assets/Enviro/Village/VR_Maison2.VR_Maison2" "/Game/_Project/Art/Assets/Enviro/Village/VR_Maison_V2_Low_Tuiles.VR_Maison_V2_Low_Tuiles"))
  (bind _output_get (Variables|Default|SetNbHabitants (Math|Random|RandomIntegerinRange (Variables|Default|GetMinHabitants) (Variables|Default|GetMaxHabitants))))
  (for _index (range 1 _output_get)
    (bind _returnvalue (Game|SpawnActorfromClass "/Game/_Project/Blueprints/Gameloop/BP_LilGuy.BP_LilGuy_C" (Transformation|GetWorldTransform (Variables|Default|GetHabitantSpawnPoint)) "AlwaysSpawn" "MultiplyWithRoot" 0 (Variables|Default|GetDefaultSpline) 0))
    (Utilities|Array|AddUnique (Variables|Default|GetHabitantsList) _returnvalue)
    (Default|OnBirth _returnvalue)))

(event EventEndOverlap
  (params (MotionController :type Motion%20Controller%20Component%20Object%20Reference))
  ;[0.15 0.15 0.15 0.5] Hand Overlap
  (Variables|Default|SetMotion%20Controller MotionController))

(event Custom|CE_BeginOverlapFB
  (CallFunction|CEPlaySoundatHouse)
  (Class|PlayerController|PlayHapticEffect (Game|GetPlayerController 0) (Variables|Default|GetOnSmashHaptic%20Effect) (select (Utilities|Name|Equal(Name) (Variables|/Script/HeadMountedDisplay.MotionControllerComponent|GetMotionSource (Variables|Default|GetMotion%20Controller)) "LeftGrip") "Left" "Right") 1.0 false))

(event Custom|CE_PlayParticleAtHouse)

(event Custom|CE_PlaySoundAtHouse
  (params (Sound :type Sound%20Base%20Object%20Reference))
  (Utilities|IsValid Sound
    (:Is%20Valid
      (Audio|PlaySoundatLocation Sound (Transformation|GetActorLocation) "0, 0, 0" 1.0 1.0 0.0 0 0 0 0))))

(fn ConstructionScript)

(fn KillAllHabitants
  (for _array_element (Variables|Default|GetHabitantsList)
    (Utilities|IsValid _array_element
      (:Is%20Valid
        (Default|OnDie _array_element))))
  (Utilities|Array|Clear (Variables|Default|GetHabitantsList)))
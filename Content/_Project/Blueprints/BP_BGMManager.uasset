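; BP_BGMManager is a background music manager that owns a single audio component for the game's music.
; On BeginPlay it starts the looping menu music and registers itself on the DataJeuDuBidou game instance so other objects can reach it.
; Events start a given sound, stop it, or pause and resume it, with the pause event also printing its state for debugging.
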(event Custom|StopBGM
  (Audio|Components|Audio|Stop (Variables|Default|GetAudio)))

(event Custom|Start%20BGM
  (params (NewSound :type Sound%20Base%20Object%20Reference))
  (bind _audio (Variables|Default|GetAudio))
  (Audio|Components|Audio|SetSound _audio NewSound)
  (Audio|Components|Audio|Play _audio 0.0))

(event Custom|PauseBGM
  (params (bPause :type Boolean))
  (Development|PrintText (Utilities|Text|FormatText "Pause {avvv}" bPause))
  (Class|AudioComponent|SetPaused (Variables|Default|GetAudio) bPause))

(event EventBeginPlay
  (CallFunction|StartBGM "/Game/_Project/Sound/BackgroundMusic/Background_MenuMusic_Loop.Background_MenuMusic_Loop")
  (bind _asdata_jeu_du_bidou (Utilities|Casting|CastToDataJeuDuBidou (Game|GetGameInstance)))
  (Variables|/Game/_Project/Data/DataJeuDuBidou.DataJeuDuBidou_C|SetBGMManager _asdata_jeu_du_bidou self))

(fn ConstructionScript)
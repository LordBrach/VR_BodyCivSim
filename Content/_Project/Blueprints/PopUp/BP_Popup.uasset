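; BP_Popup is an actor that displays a WBP_PopUp through its widget component and can be repositioned in the world.
; It caches the widget on BeginPlay, and SetupPopup passes the popup value to it, stores that value and unhides the actor.
; MoveTo restarts the Move timeline to lerp from the current location to the new one with teleporting, while RemovePopup hides the actor without destroying it.
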(event Custom|Setup%20Popup
  (params (Popup :type EN_Popup%20Enum :default "NewEnumerator0"))
  (Default|SetPopup (Variables|Default|GetAs%20WBP%20Pop%20Up) Popup)
  (Variables|Default|SetPopupValue Popup)
  (Rendering|SetActorHiddenInGame false))

(event Custom|MoveTo
  (params (NewPosition :type Vector))
  (Variables|Default|SetCurrentPosition (Transformation|GetActorLocation))
  (Utilities|FlowControl|Sequence
    (:then_0
      (bind _lerp (Timeline|Move Stop)
        (:Update
          (Transformation|SetActorLocation (Math|Vector|Lerp(Vector) (Variables|Default|GetCurrentPosition) NewPosition _lerp) false true))))
    (:then_1
      (Timeline|Move PlayFromStart))))

(event Custom|RemovePopup
  (Rendering|SetActorHiddenInGame true))

(event EventBeginPlay
  (bind _aswbp_pop_up (Utilities|Casting|CastToWBP_PopUp (UserInterface|GetWidget (Variables|Default|GetWidget))))
  (Variables|Default|SetAs%20WBP%20Pop%20Up _aswbp_pop_up))

(fn ConstructionScript)
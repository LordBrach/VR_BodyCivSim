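; Manager actor that shows and removes BP_Popup actors in two world-space rows, one for event popups and one for cycle popups.
; AddPopup and RemovePopup route by EventPopupValues, moving actors between a pool and active lists while rejecting duplicates.
; Active popups are spaced along the actor's forward vector and slide to close gaps on removal.
; BeginPlay spawns the pool and runs timed test calls; Tick draws a debug direction line.
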(event Custom|AddPopup
  (params (Popup :type EN_Popup%20Enum :default "NewEnumerator0"))
  (if (Utilities|Array|ContainsItem (Variables|Default|GetEventPopupValues) Popup)
    (bind _hasadded (CallFunction|AddEventPopup Popup))
    (if _hasadded
      (Development|PrintString "Added Popup" :!label _label))
    (else
      (bind _hasadded_2 (CallFunction|AddCyclePopup Popup))
      (if _hasadded_2
        (goto _label)))))

(event Custom|RemovePopup
  (params (Popup :type EN_Popup%20Enum :default "NewEnumerator0"))
  (if (Utilities|Array|ContainsItem (Variables|Default|GetEventPopupValues) Popup)
    (CallFunction|RemoveEventPopup Popup)
    (else
      (CallFunction|RemoveCyclePopup Popup))))

(event EventBeginPlay
  (for _index (range 0 (|GetNumEnumEntries))
    (bind _returnvalue (Game|SpawnActorfromClass "/Game/_Project/Blueprints/PopUp/BP_Popup.BP_Popup_C" (Transformation|GetActorTransform) "Undefined" "MultiplyWithRoot" 0 0))
    (Utilities|Array|Add (Variables|Default|GetBP_PopUpPool) _returnvalue)
    (Utilities|FlowControl|Delay 1.0)
    (CallFunction|AddPopup "NewEnumerator0")
    (Utilities|FlowControl|Delay 1.0)
    (CallFunction|AddPopup "NewEnumerator4")
    (Utilities|FlowControl|Delay 1.0)
    (CallFunction|AddPopup "NewEnumerator2")
    (Utilities|FlowControl|Delay 1.0)
    (CallFunction|RemovePopup "NewEnumerator0")))

(event EventTick
  (params (DeltaSeconds :type Float%20%28single-precision%29))
  (bind _returnvalue (Transformation|GetActorLocation))
  (Rendering|Debug|DrawDebugLine _returnvalue (+ _returnvalue (* (Transformation|GetActorForwardVector) 3e+01)) "(R=0.000000,G=0.129555,B=1.000000,A=1.000000)" DeltaSeconds 1.0))

(fn ConstructionScript)

(fn AddEventPopup
  (params (EventPopup :type EN_Popup%20Enum :default "NewEnumerator0"))
  (bind _bp_popuppool (Variables|Default|GetBP_PopUpPool))
  (bind _activeeventpopups (Variables|Default|GetActiveEventPopUps))
  (bind _output (Utilities|Array|Get(acopy) _bp_popuppool))
  (Utilities|FlowControl|Sequence
    (:then_0
      (for _array_element (Variables|Default|GetActiveEventPopUps)
        (if (Utilities|Enum|Equal(Enum) EventPopup (Variables|/Game/_Project/Blueprints/PopUp/BP_Popup.BP_Popup_C|GetPopupValue _array_element))
          (return false))))
    (:then_1
      (Utilities|IsValid _output
        (:Is%20Valid
          (Transformation|SetActorLocation _output (Transformation|GetWorldLocation (Variables|Default|GetEventPopups)) false true)
          (Default|SetupPopup _output EventPopup)
          (Utilities|Array|Add (Variables|Default|GetActiveEventPopUps) _output)
          (Utilities|Array|RemoveItem (Variables|Default|GetBP_PopUpPool) _output))
        (:Is%20Not%20Valid
          (return false))))
    (:then_2
      (for _index (range 1 (- (Utilities|Array|Length _activeeventpopups) 1))
        (Default|Moveto (Utilities|Array|Get(acopy) _activeeventpopups _index) (+ (Transformation|GetWorldLocation (Variables|Default|GetEventPopups)) (* (Transformation|GetActorForwardVector) (Variables|Default|GetDistanceBetweenPopups) _index))))
      (return true))))

(fn AddCyclePopup
  (params (CyclePopup :type EN_Popup%20Enum :default "NewEnumerator0"))
  (bind _bp_popuppool (Variables|Default|GetBP_PopUpPool))
  (bind _activecyclepopups (Variables|Default|GetActiveCyclePopUps))
  (bind _output (Utilities|Array|Get(acopy) _bp_popuppool))
  (Utilities|FlowControl|Sequence
    (:then_0
      (for _array_element (Variables|Default|GetActiveCyclePopUps)
        (if (Utilities|Enum|Equal(Enum) CyclePopup (Variables|/Game/_Project/Blueprints/PopUp/BP_Popup.BP_Popup_C|GetPopupValue _array_element))
          (return false))))
    (:then_1
      (Utilities|IsValid _output
        (:Is%20Valid
          (Transformation|SetActorLocation _output (Transformation|GetWorldLocation (Variables|Default|GetCyclePopUps)) false true)
          (Default|SetupPopup _output CyclePopup)
          (Utilities|Array|Add (Variables|Default|GetActiveCyclePopUps) _output)
          (Utilities|Array|RemoveItem (Variables|Default|GetBP_PopUpPool) _output))
        (:Is%20Not%20Valid
          (return false))))
    (:then_2
      (for _index (range 1 (- (Utilities|Array|Length _activecyclepopups) 1))
        (Default|Moveto (Utilities|Array|Get(acopy) _activecyclepopups _index) (+ (Transformation|GetWorldLocation (Variables|Default|GetCyclePopUps)) (* (Transformation|GetActorForwardVector) (Variables|Default|GetDistanceBetweenPopups) _index))))
      (return true))))

(fn RemoveEventPopup
  (params (Popup :type EN_Popup%20Enum :default "NewEnumerator0"))
  (bind _activeeventpopups (Variables|Default|GetActiveEventPopUps))
  (bind (_array_element _array_index) (Utilities|Array|ForEachLoopwithBreak (Variables|Default|GetActiveEventPopUps) :!label _label)
    (:LoopBody
      (if (Utilities|Enum|Equal(Enum) Popup (Variables|/Game/_Project/Blueprints/PopUp/BP_Popup.BP_Popup_C|GetPopupValue _array_element))
        (LocalVariables|SetToRemovePopup _array_element)
        (LocalVariables|SetToRemoveIndex _array_index)
        (goto _label Break)))
    (:Completed
      (Utilities|IsValid (LocalVariables|GetToRemovePopup)
        (:Is%20Valid
          (Default|RemovePopup (LocalVariables|GetToRemovePopup))
          (Utilities|Array|RemoveItem (Variables|Default|GetActiveEventPopUps) (LocalVariables|GetToRemovePopup))
          (Utilities|Array|Add (Variables|Default|GetBP_PopUpPool) (LocalVariables|GetToRemovePopup))
          (for _index (range (LocalVariables|GetToRemoveIndex) (- (Utilities|Array|Length _activeeventpopups) 1))
            (Default|Moveto (Utilities|Array|Get(acopy) _activeeventpopups _index) (+ (Transformation|GetWorldLocation (Variables|Default|GetEventPopups)) (* (Transformation|GetActorForwardVector) (Variables|Default|GetDistanceBetweenPopups) _index)))))))))

(fn RemoveCyclePopup
  (params (Popup :type EN_Popup%20Enum :default "NewEnumerator0"))
  (bind _activecyclepopups (Variables|Default|GetActiveCyclePopUps))
  (bind (_array_element _array_index) (Utilities|Array|ForEachLoopwithBreak (Variables|Default|GetActiveCyclePopUps) :!label _label)
    (:LoopBody
      (if (Utilities|Enum|Equal(Enum) Popup (Variables|/Game/_Project/Blueprints/PopUp/BP_Popup.BP_Popup_C|GetPopupValue _array_element))
        (LocalVariables|SetToRemovePopup _array_element)
        (LocalVariables|SetToRemoveIndex _array_index)
        (goto _label Break)))
    (:Completed
      (Utilities|IsValid (LocalVariables|GetToRemovePopup)
        (:Is%20Valid
          (Default|RemovePopup (LocalVariables|GetToRemovePopup))
          (Utilities|Array|RemoveItem (Variables|Default|GetActiveCyclePopUps) (LocalVariables|GetToRemovePopup))
          (Utilities|Array|Add (Variables|Default|GetBP_PopUpPool) (LocalVariables|GetToRemovePopup))
          (for _index (range (LocalVariables|GetToRemoveIndex) (- (Utilities|Array|Length _activecyclepopups) 1))
            (Default|Moveto (Utilities|Array|Get(acopy) _activecyclepopups _index) (+ (Transformation|GetWorldLocation (Variables|Default|GetCyclePopUps)) (* (Transformation|GetActorForwardVector) (Variables|Default|GetDistanceBetweenPopups) _index)))))))))
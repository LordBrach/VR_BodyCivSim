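; Hunger component that tracks a food value, drains it over time and classifies it as Full, Hungry or Starving.
; Update subtracts a time-sampled curve rate scaled by delta seconds, then UpdateState compares the value against the HungerSteps thresholds.
; Changes to Full or Hungry broadcast OnStateChanged, while entering Starving instead fires OnStarveLaunched and grants bonus food.
; AddFood is the clamped entry point for replenishment.
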(event Custom|AddFood
  (params (FoodValue :type Float%20%28double-precision%29))
  (Variables|Default|SetFoodValue (Math|Float|Clamp(Float) (+ FoodValue (Variables|Default|GetFoodValue)) 0.0 1e+02)))

(event Custom|Update
  (params (DeltaSeconds :type Float%20%28double-precision%29) (CurrentTime :type Float%20%28double-precision%29))
  (Variables|Default|SetFoodValue (Math|Float|Clamp(Float) (- (Variables|Default|GetFoodValue) (* (Math|Curves|GetFloatValue (Variables|Default|GetHungerCurve) CurrentTime) DeltaSeconds)) 0.0 1e+02))
  (bind (_newstate _haschanged) (CallFunction|UpdateState))
  (if _haschanged
    (switch Utilities|FlowControl|Switch|SwitchonEN_HungerState _newstate
      (:NewEnumerator0
        (Default|CallOnStateChanged (Variables|Default|GetHungerState) :!label _label))
      (:NewEnumerator1
        (goto _label))
      (:NewEnumerator2
        (Default|CallOnStarveLaunched)
        (Variables|Default|SetFoodValue (+ (Variables|Default|GetFoodValue) (Variables|Default|GetStarveGainedFood)))))))

(fn UpdateState
  (bind _hungersteps (Variables|Default|GetHungerSteps))
  (bind _foodvalue (Variables|Default|GetFoodValue))
  (Utilities|FlowControl|Sequence
    (:then_0
      (if (< _foodvalue (.Value (Utilities|Map|Find _hungersteps "NewEnumerator1")))
        (LocalVariables|SetState (select (< _foodvalue (.Value (Utilities|Map|Find _hungersteps "NewEnumerator2"))) "NewEnumerator2" "NewEnumerator1"))))
    (:then_1
      (bind _output_get (LocalVariables|SetBHasChanged (Utilities|Enum|NotEqual(Enum) (LocalVariables|GetState) (Variables|Default|GetHungerState))))
      (bind _output_get_2 (Variables|Default|SetHungerState (LocalVariables|GetState)))
      (return _output_get_2 _output_get))))
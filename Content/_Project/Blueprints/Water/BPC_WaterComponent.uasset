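; BPC_WaterComponent is an actor component that tracks a water gauge and maps it to five states from Dry through Regular to Tsunami.
; The gauge drains every Tick and rises through AddWater, and UpdateWater compares it against WaterSteps thresholds to detect state changes.
; Middle states broadcast a state-changed notification, while the extremes trigger Tsunami or Drought, which announce themselves and push the gauge back toward the middle.
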(event Custom|AddWater
  (params (DeltaSeconds :type Float%20%28double-precision%29))
  (Variables|Default|SetWaterJauge (+ (Variables|Default|GetWaterJauge) (* (Variables|Default|GetWaterWonSpeed) DeltaSeconds)))
  (CallFunction|UpdateWater))

(event Custom|CallTsunami
  ;[0.15 0.15 0.15 0.5] Events
  (Default|CallOnTsunamiTriggered)
  (Development|PrintString "TSUNAMIII")
  (Variables|Default|SetWaterJauge (- (Variables|Default|GetWaterJauge) (Variables|Default|GetTsunamiLostWater))))

(event Custom|CallDrought
  ;[0.15 0.15 0.15 0.5] Events
  (Default|CallOnDroughtTriggered)
  (Development|PrintString "DROUGHT!!!")
  (Variables|Default|SetWaterJauge (+ (Variables|Default|GetWaterJauge) (Variables|Default|GetDroughtGainedWater))))

(event EventTick
  (params (DeltaSeconds :type Float%20%28single-precision%29))
  (Variables|Default|SetWaterJauge (- (Variables|Default|GetWaterJauge) (* DeltaSeconds (Variables|Default|GetWaterLostSpeed))))
  (CallFunction|UpdateWater))

(fn GetStatefromJauge
  (bind _watersteps (Variables|Default|GetWaterSteps))
  (bind _waterjauge (Variables|Default|GetWaterJauge))
  (if (> _waterjauge (.Value (Utilities|Map|Find _watersteps "NewEnumerator1")))
    (return (select (> (Variables|Default|GetWaterJauge) (.Value (Utilities|Map|Find (Variables|Default|GetWaterSteps) "NewEnumerator0"))) "NewEnumerator0" "NewEnumerator1"))
    (elif (< _waterjauge (.Value (Utilities|Map|Find _watersteps "NewEnumerator2")))
      (return (select (< _waterjauge (.Value (Utilities|Map|Find _watersteps "NewEnumerator3"))) "NewEnumerator3" "NewEnumerator2"))
      (else
        (return "NewEnumerator4")))))

(fn UpdateWater
  (bind _state (CallFunction|GetStatefromJauge))
  (if (Utilities|Enum|NotEqual(Enum) _state (Variables|Default|GetCurrentState))
    (bind _output_get (Variables|Default|SetCurrentState _state))
    (switch Utilities|FlowControl|Switch|SwitchonEN_WaterState _output_get
      (:NewEnumerator4
        (Default|CallOnWaterStateChanged (Variables|Default|GetCurrentState) :!label _label))
      (:NewEnumerator0
        (CallFunction|CallTsunami))
      (:NewEnumerator1
        (goto _label))
      (:NewEnumerator2
        (goto _label))
      (:NewEnumerator3
        (CallFunction|CallDrought)))))
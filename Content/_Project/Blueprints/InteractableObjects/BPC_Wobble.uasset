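; BPC_Wobble is an actor component that makes its owning actor wobble around a base location.
; BeginPlay caches the owner and picks a random scale for each axis.
; Play and Stop events control a looping timer, set at the current frame's delta time, that drives updates in place of Tick.
; Each update offsets the base location with scaled per-axis sine waves, blends by alpha and teleports the owner there.
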(event Custom|CE_Play
  (if (not (Utilities|Time|IsTimerActivebyHandle (Variables|Default|Getth_WobbleTimer)))
    (bind _returnvalue (Utilities|Time|SetTimerbyEvent (delegate Custom|CE_StartWobbleTimer) (Utilities|Time|GetWorldDeltaSeconds) true))
    (Variables|Default|Setth_WobbleTimer _returnvalue)))

(event Custom|CE_StartWobbleTimer
  (CallFunction|CEUpdate))

(event Custom|CE_Update
  (bind _v3_initlocation (Variables|Vector|Getv3_InitLocation))
  (bind _v3_randomvector (Variables|Vector|Getv3_RandomVector))
  (Variables|Default|Setf_TimeAccumulator (+ (Variables|Default|Getf_TimeAccumulator) (* (Utilities|Time|GetWorldDeltaSeconds) (Variables|Default|Getf_Speed))))
  (Variables|Vector|Setf_SinOffSet (* (Math|Vector|MakeVector (* (Math|Trig|Sin(Radians) (.x (* (Variables|Vector|Getf_SinFrequency) (Variables|Default|Getf_TimeAccumulator)))) (.x _v3_randomvector)) (* (Math|Trig|Sin(Radians) (.y (* (Variables|Vector|Getf_SinFrequency) (Variables|Default|Getf_TimeAccumulator)))) (.y _v3_randomvector)) (* (Math|Trig|Sin(Radians) (.z (* (Variables|Vector|Getf_SinFrequency) (Variables|Default|Getf_TimeAccumulator)))) (.z _v3_randomvector))) (Variables|Vector|Getf_Amplitude)))
  (Transformation|SetActorLocation (Variables|Default|GetParentActor) (Math|Vector|Lerp(Vector) _v3_initlocation (+ _v3_initlocation (Variables|Vector|Getf_SinOffSet)) (Variables|Default|Getf_Alpha)) false true))

(event Custom|CE_Stop
  (Utilities|Time|ClearandInvalidateTimerbyHandle (Variables|Default|Getth_WobbleTimer)))

(event EventBeginPlay
  (bind _v2_randomminmax (Variables|Vector|Getv2_RandomMinMax))
  (bind _returnvalue (Math|Random|RandomFloatinRange (.x _v2_randomminmax) (.y _v2_randomminmax)))
  (Variables|Default|SetParentActor (Components|GetOwner))
  (Variables|Vector|Setv3_RandomVector (Math|Vector|MakeVector _returnvalue _returnvalue _returnvalue)))

(event EventTick
  (params (DeltaSeconds :type Float%20%28single-precision%29)))
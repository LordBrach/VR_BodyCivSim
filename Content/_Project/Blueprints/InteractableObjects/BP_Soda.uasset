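; BP_Soda is a grabbable soda that drips when tipped and spills onto actors below it.
; Grab and drop events toggle Tick, which activates the drip component once absolute mesh roll exceeds 90 degrees.
; While dripping, a downward line trace sends AddWater with delta time to the hit actor.
; Reset zeroes physics velocities and restores the mesh transform saved at BeginPlay.
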(event OnGrabbed(GrabComponent)
  (params (MotionController :type Motion%20Controller%20Component%20Object%20Reference))
  (Actor|Tick|SetActorTickEnabled true))

(event OnDropped(GrabComponent)
  (Actor|Tick|SetActorTickEnabled false)
  (Components|Activation|Deactivate (Variables|Default|GetDrippingSoda))
  (Variables|Default|SetIsDripping false))

(event EventBeginPlay
  (Variables|Default|SetBeginTransform (Transformation|GetRelativeTransform (Variables|Default|GetSodaMesh))))

(event EventTick
  (params (DeltaSeconds :type Float%20%28single-precision%29))
  (bind _drippingsoda (Variables|Default|GetDrippingSoda))
  (bind _sodamesh (Variables|Default|GetSodaMesh))
  (bind _drippingsoda_2 (Variables|Default|GetDrippingSoda))
  (bind _returnvalue (Transformation|GetWorldRotation _sodamesh))
  (bind _returnvalue_2 (Transformation|GetWorldLocation _drippingsoda_2))
  (bind _returnvalue_3 (Math|Float|Absolute(Float) (.roll _returnvalue)))
  (bind _returnvalue_4 (Math|Float|Absolute(Float) (.roll _returnvalue)))
  (bind _returnvalue_5 (> _returnvalue_4 -9e+01))
  (bind _returnvalue_6 (> _returnvalue_3 9e+01))
  (bind _returnvalue_7 (Class|KismetMathLibrary|XORBoolean _returnvalue_5 _returnvalue_6))
  (bind _returnvalue_8 (not _returnvalue_7))
  ;[0.15 0.15 0.15 0.5] Dripping Detection
  (Utilities|FlowControl|Sequence
    (:then_0
      (if (!= (Variables|Default|GetIsDripping) _returnvalue_8)
        (bind _output_get (Variables|Default|SetIsDripping _returnvalue_8))
        (if _output_get
          (Components|Activation|Activate _drippingsoda true)
          (Development|PrintString "activate")
          (else
            (Components|Activation|Deactivate _drippingsoda)
            (Development|PrintString "deactivate")))))
    (:then_1
      ;[0.15 0.15 0.15 0.5] Detection of Spilled Area
      (if (Variables|Default|GetIsDripping)
        (bind (_outhit _returnvalue_9) (Collision|LineTraceByChannel _returnvalue_2 (+ _returnvalue_2 "0.000000,0.000000,-500.000000") "TraceTypeQuery4" false 0 "None"))
        (if _returnvalue_9
          (Class|INWaterSensible|AddWater(Message) (.HitActor (Collision|BreakHitResult _outhit)) DeltaSeconds))))))

(event EventReset
  (bind _sodamesh (Variables|Default|GetSodaMesh))
  (Physics|SetPhysicsLinearVelocity _sodamesh "0, 0, 0" false "None")
  (Class|PrimitiveComponent|SetPhysicsAngularVelocityinDegrees _sodamesh "0, 0, 0" false "None")
  (Transformation|SetRelativeTransform _sodamesh (Variables|Default|GetBeginTransform) false false)
  (Development|PrintString "RESET" true true "(R=0.000000,G=0.000000,B=0.000000,A=1.000000)" 1e+02))

(fn ConstructionScript)
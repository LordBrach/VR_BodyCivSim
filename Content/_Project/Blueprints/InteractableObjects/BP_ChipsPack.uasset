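; BP_ChipsPack is a grabbable VR chips pack that hands out individual chips instead of being held itself.
; When grabbed, it stores the motion controller, releases itself and gives that controller the first available chip from a pre-made ChipPool, printing a message if none remain.
; When the pack's grab component drops, it releases and clears the held chip.
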(event OnGrabbed(GrabComponent)
  (params (MotionController :type Motion%20Controller%20Component%20Object%20Reference))
  (bind _grabcomponent (Variables|Default|GetGrabComponent))
  (Variables|Default|SetMotion%20Controller%20Ref (Variables|/Game/VRTemplate/Blueprints/GrabComponent.GrabComponent_C|GetMotionControllerRef _grabcomponent))
  (Default|TryRelease _grabcomponent)
  (bind _success (CallFunction|TakeChipsfromPool))
  (if (not _success)
    (Development|PrintString "NO CHIPS AVAILABLE")))

(event OnDropped(GrabComponent)
  (bind _heldchips (Variables|Default|GetHeldChips)
    (:then
      (Default|TryRelease (Variables|/Game/_Project/Blueprints/InteractableObjects/BP_Chips.BP_Chips_C|GetGrabComponent _heldchips))
      (Variables|Default|SetHeldChips 0))
    (:else)))

(event EventBeginPlay)

(fn ConstructionScript)

(fn TakeChipsfromPool
  (for _array_element (Variables|Default|GetChipPool)
    (if (Default|IsinPool _array_element)
      (Default|TakeChips _array_element (Variables|Default|GetMotion%20Controller%20Ref))
      (Variables|Default|SetHeldChips _array_element)
      (return true)))
  (return false))
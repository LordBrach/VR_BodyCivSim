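; VR fly that buzzes around the player's head until swatted with a motion controller.
; Tick offsets the fly mesh on a per-axis sine wave around the last sampled camera position, with looping logic replaced by an interpolated actor move once the meteorite timer expires.
; A fast enough controller overlap plays sound, Niagara and per-hand haptic feedback, then re-initializes the fly with random scale and wave phase.
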(event Custom|CE_Init
  (Rendering|SetActorHiddenInGame false)
  (Variables|Init|Setv3_InitScale (* "0.050000,0.050000,0.050000" (Math|Random|RandomFloatinRange 0.75 1.25)))
  (Transformation|SetWorldScale3D (Variables|Default|GetFlie) (Variables|Init|Getv3_InitScale))
  (Variables|RandomLevitate|Setf_TimeAccumulator (Math|Random|RandomFloatinRange 0.0 5e+02))
  (Variables|Default|Setf_MeteoriteTimer 0.0))

(event Custom|CE_FlieDisappear
  (Utilities|Time|ClearandInvalidateTimerbyHandle (Variables|Default|Getth_MeteoriteTimer))
  (CallFunction|CEFlieDisappearFB)
  (CallFunction|CEInit))

(event Custom|CE_FlyAround
  (if (not (Variables|Rendering|GetbHidden))
    (Variables|RandomLevitate|Setf_TimeAccumulator (+ (Variables|RandomLevitate|Getf_TimeAccumulator) (* (Utilities|Time|GetWorldDeltaSeconds) (Variables|RandomLevitate|Getf_FartSpeed))))
    (Variables|RandomLevitate|Setf_SinOffSet (* (Math|Vector|MakeVector (Math|Trig|Sin(Radians) (.x (* (Variables|RandomLevitate|Getf_SinFrequency) (Variables|RandomLevitate|Getf_TimeAccumulator)))) (Math|Trig|Sin(Radians) (.y (* (Variables|RandomLevitate|Getf_SinFrequency) (Variables|RandomLevitate|Getf_TimeAccumulator)))) (Math|Trig|Sin(Radians) (.z (* (Variables|RandomLevitate|Getf_SinFrequency) (Variables|RandomLevitate|Getf_TimeAccumulator))))) (Variables|RandomLevitate|Getf_Amplitude)))
    (Transformation|SetWorldLocation (Variables|Default|GetFlie) (+ (Variables|Init|Getv3_InitLocation) (Variables|RandomLevitate|Getf_SinOffSet)) false true)
    (Variables|Init|Setv3_InitLocation (Transformation|GetWorldLocation (Variables|/Game/_Project/Blueprints/Player/VRPawnPlayer.VRPawnPlayer_C|GetCamera (Variables|Default|GetAs%20VRPawn%20Player))))
    (CallFunction|CEPlaySoundatFlie (Variables|Feedback|GetFlieFlyingSound))))

(event EventBeginPlay
  (bind _asvrpawn_player (Utilities|Casting|CastToVRPawnPlayer (Game|Player|GetPlayerPawn 0)))
  (Variables|Default|SetAs%20VRPawn%20Player _asvrpawn_player)
  (CallFunction|CEInit))

(event Collision|EventActorBeginOverlap
  (params (OtherActor :type Actor%20Object%20Reference)))

(event EventTick
  (params (DeltaSeconds :type Float%20%28single-precision%29))
  (if (not (Variables|Rendering|GetbHidden))
    (Variables|Default|Setf_MeteoriteTimer (+ (Variables|Default|Getf_MeteoriteTimer) (Utilities|Time|GetWorldDeltaSeconds)))
    (if (> (Variables|Default|Getf_MeteoriteTimer) (Variables|Default|Getf_MeteoriteCD))
      (Transformation|SetActorLocation (Math|Interpolation|VInterpTo (Transformation|GetActorLocation) "0, 0, 0" (Utilities|Time|GetWorldDeltaSeconds) (Variables|Default|Getf_MeteoriteInterSpeed)) false true)
      (else
        (CallFunction|CEFlyAround)))))

(event EventEndOverlap
  (params (MotionController :type Motion%20Controller%20Component%20Object%20Reference))
  (Variables|Default|SetcurrentMotionController 0))

(event EventBeginOverlap
  (params (MotionController :type Motion%20Controller%20Component%20Object%20Reference))
  (Variables|Default|SetcurrentMotionController MotionController)
  (if (> (Math|Vector|VectorLength (.OutLinearVelocity (Class|MotionControllerComponent|GetLinearVelocity (Variables|Default|GetcurrentMotionController)))) (Variables|Default|Getf_SmashForce))
    (CallFunction|CEFlieDisappear)))

(event Custom|CE_InitFB
  (CallFunction|CEPlaySoundatFlie (Variables|Feedback|GetOnFlieSpawnSound))
  (CallFunction|CEPlayParticleatFlie (Variables|Feedback|GetOnFlieSpawnParticle)))

(event Custom|CE_PlaySoundAtFlie
  (params (Sound :type Sound%20Base%20Object%20Reference))
  (Utilities|IsValid Sound
    (:Is%20Valid
      (Audio|PlaySoundatLocation Sound (Transformation|GetActorLocation) "0, 0, 0" 1.0 1.0 0.0 0 0 0 0))))

(event Custom|CE_FlieDisappearFB
  (CallFunction|CEPlaySoundatFlie (Variables|Feedback|GetFlieDisappearSound))
  (Class|PlayerController|PlayHapticEffect (Game|GetPlayerController 0) (Variables|Feedback|GetFlieDisappear%20Haptic%20Effect) (select (Utilities|Name|Equal(Name) (Variables|/Script/HeadMountedDisplay.MotionControllerComponent|GetMotionSource (Variables|Default|GetcurrentMotionController)) "LeftGrip") "Left" "Right") 1.0 false)
  (CallFunction|CEPlayParticleatFlie (Variables|Feedback|GetOnFlieDisappearParticle)))

(event Custom|CE_PlayParticleAtFlie
  (params (InAsset :type Niagara%20System%20Object%20Reference))
  (bind _niagara (Variables|Default|GetNiagara))
  (Utilities|IsValid InAsset
    (:Is%20Valid
      (Class|NiagaraComponent|SetAsset _niagara InAsset true)
      (Components|Activation|Activate _niagara false))))

(fn ConstructionScript)
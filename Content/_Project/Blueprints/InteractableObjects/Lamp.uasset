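; VR lamp with a pull-down switch that toggles its point light on and off when grabbed and pulled far enough.
; While grabbed, Tick moves the switch vertically with the motion controller's height change, clamped between TargetPos and its height at grab.
; Reaching TargetPos toggles the light and forces a release.
; On release, a timeline lerps the switch back to its origin, and a new grab interrupts that return.
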(event OnGrabbed(GrabComponent)
  (Variables|Default|SetOnGrabHandPos (Transformation|GetWorldLocation (Variables|/Game/VRTemplate/Blueprints/GrabComponent.GrabComponent_C|GetMotionControllerRef (Variables|Default|GetGrabComponent))))
  (Variables|Default|SetOnGrabInterruptorPos (Transformation|GetWorldLocation (Variables|Default|GetInterruptor)))
  (Actor|Tick|SetActorTickEnabled true)
  (CallFunction|StopTimeline))

(event OnDropped(GrabComponent)
  (Actor|Tick|SetActorTickEnabled false)
  (CallFunction|ReplaceInterruptor))

(event Custom|ReplaceInterruptor
  (Variables|Default|SetTempPos (Transformation|GetWorldLocation (Variables|Default|GetInterruptor)))
  (bind _lerp (Timeline|InterruptorTimeline PlayFromStart)
    (:Update
      (Transformation|SetWorldLocation (Variables|Default|GetInterruptor) (Math|Vector|Lerp(Vector) (Variables|Default|GetTempPos) (Variables|Default|GetInterruptorOrigin) _lerp) false false))))

(event Custom|StopTimeline
  (bind _lerp (Timeline|InterruptorTimeline Stop)
    (:Update
      (Transformation|SetWorldLocation (Variables|Default|GetInterruptor) (Math|Vector|Lerp(Vector) (Variables|Default|GetTempPos) (Variables|Default|GetInterruptorOrigin) _lerp) false false))))

(event EventBeginPlay
  (Variables|Default|SetInterruptorOrigin (Transformation|GetWorldLocation (Variables|Default|GetInterruptor))))

(event EventTick
  (params (DeltaSeconds :type Float%20%28single-precision%29))
  (bind _ongrabhandpos (Variables|Default|GetOnGrabHandPos))
  (bind _grabcomponent (Variables|Default|GetGrabComponent))
  (bind _interruptor (Variables|Default|GetInterruptor))
  (bind _ongrabinterruptorpos (Variables|Default|GetOnGrabInterruptorPos))
  (bind _targetpos (Variables|Default|GetTargetPos))
  (bind _returnvalue (Transformation|GetWorldLocation _targetpos))
  (bind _motioncontrollerref (Variables|/Game/VRTemplate/Blueprints/GrabComponent.GrabComponent_C|GetMotionControllerRef _grabcomponent))
  (bind _returnvalue_2 (Transformation|GetWorldLocation _motioncontrollerref))
  (bind _returnvalue_3 (- (.z _returnvalue_2) (.z _ongrabhandpos)))
  (bind _returnvalue_4 (+ _returnvalue_3 (.z _ongrabinterruptorpos)))
  (Development|PrintString (Utilities|String|ToString(Float) _returnvalue_4) true true "(R=0.000000,G=0.660000,B=1.000000,A=1.000000)" DeltaSeconds)
  (Transformation|SetWorldLocation _interruptor (Math|Vector|MakeVector (.x _ongrabinterruptorpos) (.y _ongrabinterruptorpos) (Math|Float|Clamp(Float) _returnvalue_4 (.z _returnvalue) (.z _ongrabinterruptorpos))) false true)
  (if (<= (.z (Transformation|GetWorldLocation _interruptor)) (.z _returnvalue))
    (CallFunction|SwitchLight)
    (Default|TryRelease (Variables|Default|GetGrabComponent))
    (CallFunction|ReplaceInterruptor)))

(fn ConstructionScript)

(fn SwitchLight
  (bind _output_get (Variables|Default|SetIsOn (not (Variables|Default|GetIsOn))))
  (Rendering|Components|Light|SetIntensity (Variables|Default|GetPointLight) (Math|Float|SelectFloat 5e+03 0.0 _output_get)))
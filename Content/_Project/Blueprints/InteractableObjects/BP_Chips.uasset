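; BP_Chips is a pooled, grabbable food item that a motion controller can take and eat.
; Taking it unhides the actor and grabs it through GrabComponent, while eating plays a spatialized sound, releases the grab and hides it again.
; The hidden flag doubles as the pool-availability state, Reset returns the item by hiding it, and GetFoodValue exposes its food value.
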(event Custom|TakeChips
  (params (MotionController :type Motion%20Controller%20Component%20Object%20Reference))
  (Rendering|SetActorHiddenInGame false)
  (Default|TryGrab (Variables|Default|GetGrabComponent) MotionController))

(event EventBeginPlay)

(event EventEat
  (Default|PlaySoundSpatialized (Variables|Default|GetBPC_SoundPlayer) "EatChips")
  (Default|TryRelease (Variables|Default|GetGrabComponent))
  (Rendering|SetActorHiddenInGame true)
  (Development|PrintString "EATTTTT"))

(event EventReset
  (Rendering|SetActorHiddenInGame true))

(fn ConstructionScript)

(fn IsinPool
  (return (Variables|Rendering|GetbHidden)))

(fn GetFoodValue
  (return (Variables|Default|GetFoodValue)))
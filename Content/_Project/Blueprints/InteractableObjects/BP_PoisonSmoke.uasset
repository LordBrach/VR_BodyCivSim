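; VR interactable poison (fart) smoke cloud that the player disperses by waving motion controllers inside it.
; Tick bobs the randomly scaled smoke around its origin with accumulated-time sine offsets.
; While controllers overlap, a looping timer converts their linear velocity into health damage, shrinking the smoke with per-hand haptics and sound.
; Depleted health triggers disappearance sound, haptics and Niagara burst, then immediately reinitializes the cloud in place.
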(event Custom|CE_OnOverlap
  (Variables|Overlap|Setf_MotionVelocityLength 0.0)
  (for _array_element (Variables|Motion|GetMotion%20Controllers)
    (Variables|Default|SetcurrentMotionController _array_element)
    (Variables|Overlap|Setf_MotionVelocityLength (+ (Variables|Overlap|Getf_MotionVelocityLength) (Math|Vector|VectorLength (.OutLinearVelocity (Class|MotionControllerComponent|GetLinearVelocity (Variables|Default|GetcurrentMotionController))))))
    (Variables|Alpha|Setf_HandShakeAlpha (Math|Float|Clamp(Float) (Math|Float|NormalizetoRange (Variables|Overlap|Getf_MotionVelocityLength) (Variables|Var|Getf_ShakeMinValue) (Variables|Var|Getf_ShakeMaxValue))))
    (Variables|Var|Setf_FartHealth (- (Variables|Var|Getf_FartHealth) (Variables|Alpha|Getf_HandShakeAlpha)))
    (Variables|Alpha|Setf_FartHealthAlpha (Math|Float|NormalizetoRange (Variables|Var|Getf_FartHealth) 0.0 (Variables|Var|Getf_FartMaxHealth)))
    (CallFunction|CEonOverlapFB)
    (if (< (Variables|Var|Getf_FartHealth) 0.0)
      (CallFunction|CEFartDisappear))))

(event Custom|CE_Init
  (Rendering|SetActorHiddenInGame false)
  (Variables|Var|Setf_FartHealth (Variables|Var|Getf_FartMaxHealth))
  (Variables|Init|Setv3_InitScale (* "1.000000,1.000000,1.000000" (Math|Random|RandomFloatinRange 0.75 1.25)))
  (Transformation|SetWorldScale3D (Variables|Default|GetSmoke) (Variables|Init|Getv3_InitScale))
  (Variables|Init|Setv3_InitLocation (Transformation|GetActorLocation))
  (Variables|RandomLevitate|Setf_TimeAccumulator 0.0))

(event Custom|CE_FartDisappear
  (CallFunction|CEFartDisappearFB)
  (CallFunction|CEInit))

(event EventBeginPlay
  (CallFunction|CEInit))

(event Collision|EventActorBeginOverlap
  (params (OtherActor :type Actor%20Object%20Reference)))

(event EventTick
  (params (DeltaSeconds :type Float%20%28single-precision%29))
  (if (not (Variables|Rendering|GetbHidden))
    (Variables|RandomLevitate|Setf_TimeAccumulator (+ (Variables|RandomLevitate|Getf_TimeAccumulator) (* (Utilities|Time|GetWorldDeltaSeconds) (Variables|RandomLevitate|Getf_FartSpeed))))
    (Variables|RandomLevitate|Setf_SinOffSet (* (Math|Vector|MakeVector (Math|Trig|Sin(Radians) (.x (* (Variables|RandomLevitate|Getf_SinFrequency) (Variables|RandomLevitate|Getf_TimeAccumulator)))) (Math|Trig|Sin(Radians) (.y (* (Variables|RandomLevitate|Getf_SinFrequency) (Variables|RandomLevitate|Getf_TimeAccumulator)))) (Math|Trig|Sin(Radians) (.z (* (Variables|RandomLevitate|Getf_SinFrequency) (Variables|RandomLevitate|Getf_TimeAccumulator))))) (Variables|RandomLevitate|Getf_Amplitude)))
    (Transformation|SetWorldLocation (Variables|Default|GetSmoke) (+ (Variables|Init|Getv3_InitLocation) (Variables|RandomLevitate|Getf_SinOffSet)) false true)))

(event EventBeginOverlap
  (params (MotionController :type Motion%20Controller%20Component%20Object%20Reference))
  (Utilities|Array|AddUnique (Variables|Motion|GetMotion%20Controllers) MotionController)
  (if (not (Utilities|Time|IsValidTimerHandle (Variables|Overlap|Getth_OnOverlapTimer)))
    (bind _returnvalue (Utilities|Time|SetTimerbyEvent (delegate Custom|CE_OnOverlap) (Utilities|Time|GetWorldDeltaSeconds) true))
    (Variables|Overlap|Setth_OnOverlapTimer _returnvalue)))

(event EventEndOverlap
  (params (MotionController :type Motion%20Controller%20Component%20Object%20Reference))
  (Utilities|Array|RemoveItem (Variables|Motion|GetMotion%20Controllers) MotionController)
  (if (not (> (Utilities|Array|Length (Variables|Motion|GetMotion%20Controllers)) 0))
    (Utilities|Time|ClearandInvalidateTimerbyHandle (Variables|Overlap|Getth_OnOverlapTimer))))

(event Custom|CE_OnOverlapFB
  (bind _v3_initscale (Variables|Init|Getv3_InitScale))
  (Transformation|SetWorldScale3D (Variables|Default|GetSmoke) (Math|Vector|Lerp(Vector) (* _v3_initscale 0.25) _v3_initscale (Variables|Alpha|Getf_FartHealthAlpha)))
  (Class|PlayerController|PlayHapticEffect (Game|GetPlayerController 0) (Variables|Feedback|GetHandShakeHapticEffect) (select (Utilities|Name|Equal(Name) (Variables|/Script/HeadMountedDisplay.MotionControllerComponent|GetMotionSource (Variables|Default|GetcurrentMotionController)) "LeftGrip") "Left" "Right") (Variables|Alpha|Getf_HandShakeAlpha) false)
  (CallFunction|CEPlaySoundatHand (Variables|Feedback|GetOnOverlapSound)))

(event Custom|CE_PlaySoundAtHand
  (params (Sound :type Sound%20Base%20Object%20Reference))
  (Utilities|IsValid Sound
    (:Is%20Valid
      (Audio|PlaySoundatLocation Sound (Transformation|GetWorldLocation (Variables|Default|GetcurrentMotionController)) "0, 0, 0" 1.0 1.0 0.0 0 0 0 0))))

(event Custom|CE_FartDisappearFB
  (CallFunction|CEPlaySoundatHand (Variables|Feedback|GetFartDisappearSound))
  (Class|PlayerController|PlayHapticEffect (Game|GetPlayerController 0) (Variables|Feedback|GetFartDisappear%20Haptic%20Effect) (select (Utilities|Name|Equal(Name) (Variables|/Script/HeadMountedDisplay.MotionControllerComponent|GetMotionSource (Variables|Default|GetcurrentMotionController)) "LeftGrip") "Left" "Right") 1.0 false)
  (CallFunction|CEPlayParticleatSmoke (Variables|Feedback|GetOnFartDisappearParticle)))

(event Custom|CE_InitFB
  (CallFunction|CEPlaySoundatSmoke (Variables|Feedback|GetOnSmokeSpawnSound))
  (CallFunction|CEPlayParticleatSmoke (Variables|Feedback|GetOnFartSpawnParticle)))

(event Custom|CE_PlaySoundAtSmoke
  (params (Sound :type Sound%20Base%20Object%20Reference))
  (Utilities|IsValid Sound
    (:Is%20Valid
      (Audio|PlaySoundatLocation Sound (Transformation|GetActorLocation) "0, 0, 0" 1.0 1.0 0.0 0 0 0 0))))

(event Custom|CE_PlayParticleAtSmoke
  (params (InAsset :type Niagara%20System%20Object%20Reference))
  (bind _niagara (Variables|Default|GetNiagara))
  (Utilities|IsValid InAsset
    (:Is%20Valid
      (Class|NiagaraComponent|SetAsset _niagara InAsset true)
      (Components|Activation|Activate _niagara false))))

(fn ConstructionScript)
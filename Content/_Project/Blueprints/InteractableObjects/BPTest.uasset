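; BPTest is a test interactable actor that visualizes water level and day/night state.
; AddWater forwards to its water component, and Tick scales Cube1's height in proportion to that component's water gauge.
; Daylight system events swap the Sphere's material between day and night, or repeatedly print an error message when a daylight error fires.
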(event OnDayChanged(BPC_DaylightSystem)
  (params (IsDay :type Boolean))
  (Rendering|Material|SetMaterial (Variables|Default|GetSphere) 0 (select IsDay "/Engine/VREditor/UI/ArrowMaterial.ArrowMaterial" "/Engine/BufferVisualization/Anisotropy.Anisotropy")))

(event OnDaylightError(BPC_DaylightSystem)
  (for _index (range 0 10)
    (Development|PrintString "ERRRRORRRRR")))

(event EventBeginPlay)

(event EventTick
  (params (DeltaSeconds :type Float%20%28single-precision%29))
  (Transformation|SetWorldScale3D (Variables|Default|GetCube1) (Math|Vector|MakeVector 1.0 1.0 (Math|Float|Lerp 0.0 2.0 (/ (Variables|/Game/_Project/Blueprints/Water/BPC_WaterComponent.BPC_WaterComponent_C|GetWaterJauge (Variables|Default|GetBPC_WaterComponent)) 1e+02)))))

(event EventAddWater
  (params (DeltaTime :type Float%20%28double-precision%29))
  (Default|AddWater (Variables|Default|GetBPC_WaterComponent) DeltaTime))

(fn ConstructionScript)
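; VR interactable mushroom that the player grabs and pulls along its up axis until it releases and resets.
; Hand displacement over the pull distance builds an alpha that carries over between grabs.
; That alpha eases a stretch-and-thin scale and haptic strength, alongside sound and Niagara feedback for grab, hold and pull.
; Near full alpha it forces release, plays pull feedback and re-initializes with a random scale.
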(event OnGrabbed(GrabComponent)
  (params (MotionController :type Motion%20Controller%20Component%20Object%20Reference))
  (Variables|Default|SetMotion%20Controller MotionController)
  (Variables|Init|Setv3_InitialLocation (Transformation|GetWorldLocation (Variables|Default|GetMotion%20Controller)))
  (CallFunction|CEonGrabbedFB))

(event OnDropped(GrabComponent)
  (Variables|Default|SetMotion%20Controller 0)
  (Variables|Default|Setf_CurrentAlpha (Variables|Default|Getf_Alpha)))

(event OnHold(GrabComponent)
  (bind _returnvalue (Transformation|GetActorUpVector))
  (bind _motion_controller (Variables|Default|GetMotion%20Controller))
  (bind _v3_initiallocation (Variables|Init|Getv3_InitialLocation))
  (bind _returnvalue_2 (Transformation|GetWorldLocation _motion_controller))
  (bind _returnvalue_3 (- _returnvalue_2 _v3_initiallocation))
  (bind _returnvalue_4 (Math|Vector|DotProduct _returnvalue _returnvalue_3))
  (if (>= _returnvalue_4 0.0)
    (Variables|Default|Setf_Alpha (+ (Variables|Default|Getf_CurrentAlpha) (Math|Float|Clamp(Float) (Math|Float|NormalizetoRange _returnvalue_4 0.0 (Variables|Default|Getf_PullDistance)))))
    (CallFunction|CDonHoldFB)
    (if (>= (Variables|Default|Getf_Alpha) 0.9)
      (CallFunction|CEonPull))))

(event Custom|CE_Init
  (bind _returnvalue (Math|Random|RandomFloatinRange 0.5 1.0))
  (Transformation|SetWorldScale3D (Variables|Default|GetChampignon) (Math|Vector|MakeVector _returnvalue _returnvalue (Math|Random|RandomFloatinRange 0.75 1.0)))
  (Variables|Init|Setv3_InitScale (Transformation|GetWorldScale (Variables|Default|GetChampignon)))
  (Variables|Default|Setf_Alpha 0.0)
  (Variables|Default|Setf_CurrentAlpha 0.0))

(event Custom|CE_OnPull
  (Default|TryRelease (Variables|Default|GetGrabComponent))
  (CallFunction|CEonPullFB)
  (CallFunction|CEInit))

(event EventBeginPlay
  (CallFunction|CEInit))

(event Collision|EventActorBeginOverlap
  (params (OtherActor :type Actor%20Object%20Reference)))

(event EventTick
  (params (DeltaSeconds :type Float%20%28single-precision%29)))

(event Custom|CE_OnGrabbedFB
  (CallFunction|CEPlaySoundatHand (Variables|FeedBack|GetOnGrabbedSound))
  (CallFunction|CEPlayParticleatMushroom (Variables|FeedBack|GetOnGrabbedParticle)))

(event Custom|CD_OnHoldFB
  (bind _v3_initscale (Variables|Init|Getv3_InitScale))
  (bind _returnvalue (/ (.x _v3_initscale) 2.0))
  (Transformation|SetWorldScale3D (Variables|Default|GetChampignon) (Math|Vector|Lerp(Vector) (Variables|Init|Getv3_InitScale) (Math|Vector|MakeVector _returnvalue _returnvalue (* (.z _v3_initscale) 2.0)) (Math|Interpolation|Ease "EaseIn" (Variables|Default|Getf_Alpha) 0.0 1.0 4.0)))
  (Class|PlayerController|PlayHapticEffect (Game|GetPlayerController 0) (Variables|FeedBack|GetOnHoldHapticEffect) (Default|GetHeldbyHand (Variables|Default|GetGrabComponent)) (Math|Interpolation|Ease "EaseInOut" (Variables|Default|Getf_Alpha) 0.0 1.0 3.5) false)
  (CallFunction|CEPlaySoundatHand (Variables|FeedBack|GetOnHoldSound))
  (CallFunction|CEPlayParticleatMushroom (Variables|FeedBack|GetOnHoldParticle)))

(event Custom|CE_OnPullFB
  (Class|PlayerController|PlayHapticEffect (Game|GetPlayerController 0) (Variables|FeedBack|GetOnPullHapticEffect) (Default|GetHeldbyHand (Variables|Default|GetGrabComponent)) 1.0 false)
  (CallFunction|CEPlaySoundatHand (Variables|FeedBack|GetOnPullSound))
  (CallFunction|CEPlayParticleatMushroom (Variables|FeedBack|GetOnPullParticle)))

(event Custom|CE_PlaySoundAtHand
  (params (Sound :type Sound%20Base%20Object%20Reference))
  (Utilities|IsValid Sound
    (:Is%20Valid
      (Audio|PlaySoundatLocation Sound (Transformation|GetWorldLocation (Variables|Default|GetMotion%20Controller)) "0, 0, 0" 1.0 1.0 0.0 0 0 0 0))))

(event Custom|CE_PlayParticleAtMushroom
  (params (InAsset :type Niagara%20System%20Object%20Reference))
  (bind _niagara (Variables|Default|GetNiagara))
  (Utilities|IsValid InAsset
    (:Is%20Valid
      (Class|NiagaraComponent|SetAsset _niagara InAsset true)
      (Components|Activation|Activate _niagara false))))

(fn ConstructionScript)
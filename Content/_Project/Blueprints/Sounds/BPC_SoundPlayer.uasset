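; Actor component that plays sounds by name from a DataTable, either as 2D, at the owner's location, or as controllable loops.
; On BeginPlay, it binds each LoopSounds key to the owner's AudioComponent of the same name, or adds one, and assigns the table's sound.
; Start and stop functions drive those components by name.
; Names missing from the table print a red error when looked up, and missing loop entries are removed.
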(event EventBeginPlay
  (CallFunction|SetupLoopSounds))

(fn PlaySound2D
  (params (SoundName :type Name))
  (bind _returnvalue (Utilities|GetDataTableRow (Variables|Default|GetSoundsDatatable) SoundName)
    (:then
      (Audio|PlaySound2D (Utilities|Struct|BreakST_Sounds _returnvalue) 1.0 1.0 0.0 0 0))
    (:RowNotFound
      (Development|PrintString (Utilities|String|Append "Sound : \"" (Utilities|String|ToString(Name) SoundName) "\" was not found on Datatable !") true true "(R=1.000000,G=0.000000,B=0.000000,A=1.000000)"))))

(fn PlaySoundSpatialized
  (params (SoundName :type Name))
  (bind _returnvalue (Utilities|GetDataTableRow (Variables|Default|GetSoundsDatatable) SoundName)
    (:then
      (Audio|PlaySoundatLocation (Utilities|Struct|BreakST_Sounds _returnvalue) (Transformation|GetActorLocation (Components|GetOwner)) "0, 0, 0" 1.0 1.0 0.0 0 0 0 0))
    (:RowNotFound
      (Development|PrintString (Utilities|String|Append "Sound : \"" (Utilities|String|ToString(Name) SoundName) "\" was not found on Datatable !") true true "(R=1.000000,G=0.000000,B=0.000000,A=1.000000)"))))

(fn SetupLoopSounds
  (bind _loopsounds (Variables|Default|GetLoopSounds))
  (bind _loopsounds_2 (Variables|Default|GetLoopSounds))
  (if (Utilities|Map|IsNotEmpty (Variables|Default|GetLoopSounds))
    (LocalVariables|SetAudioComponents (Actor|GetComponentsByClass (Components|GetOwner) "/Script/Engine.AudioComponent"))
    (bind _keypin (Utilities|Map|ForEachLoop(Map) _loopsounds_2)
      (:then
        (bind _returnvalue (Utilities|GetDataTableRow (Variables|Default|GetSoundsDatatable) _keypin)
          (:then
            (if (.HasFound (CallFunction|GetAudioCompfromName (LocalVariables|GetAudioComponents) _keypin))
              (Utilities|Map|Add _loopsounds _keypin (.AudioComponent (CallFunction|GetAudioCompfromName (LocalVariables|GetAudioComponents) _keypin)))
              (Audio|Components|Audio|SetSound (.AudioComponent (CallFunction|GetAudioCompfromName (LocalVariables|GetAudioComponents) _keypin)) (Utilities|Struct|BreakST_Sounds _returnvalue))
              (else
                (bind _returnvalue_2 (Game|AddComponentbyClass (Components|GetOwner) "/Script/Engine.AudioComponent" false))
                (Utilities|Map|Add _loopsounds _keypin _returnvalue_2)
                (Audio|Components|Audio|SetSound _returnvalue_2 (Utilities|Struct|BreakST_Sounds _returnvalue)))))
          (:RowNotFound
            (Utilities|Map|Remove _loopsounds_2 _keypin)
            (Development|PrintString (Utilities|String|Append "Sound : \"" (Utilities|String|ToString(Name) _keypin) "\" was not found on Datatable !") true true "(R=1.000000,G=0.000000,B=0.000000,A=1.000000)")))))))

(fn GetAudioCompfromName
  (params (AudioComponents :type Array%20of%20Audio%20Component%20Object%20References) (SoundName :type Name))
  (for _array_element AudioComponents
    (if (== (Utilities|GetObjectName _array_element) SoundName)
      (return true _array_element)))
  (return false 0))

(fn StartLoopSound
  (params (SoundName :type Name))
  (Audio|Components|Audio|Play (.Value (Utilities|Map|Find (Variables|Default|GetLoopSounds) SoundName)) 0.0))

(fn StopLoopSound
  (params (SoundName :type Name))
  (Audio|Components|Audio|Stop (.Value (Utilities|Map|Find (Variables|Default|GetLoopSounds) SoundName))))
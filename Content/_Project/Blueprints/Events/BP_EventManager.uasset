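; Event manager that owns an array of event spawners and triggers random or specific game events.
; On BeginPlay it initializes every spawner, then registers itself on the DataJeuDuBidou game instance and binds TrySpawnEvent to its random-event call.
; TrySpawnEvent fires a randomly picked spawner.
; SpawnSpecificEvent force-spawns every spawner whose class exactly matches the one passed in.
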(event Custom|TrySpawnEvent
  ;[0.15 0.15 0.15 0.5] Call for one of the event spawners to do their thing (I:E, spawn an event)
  (if (Utilities|Array|IsNotEmpty (Variables|Default|GetEvents))
    (Default|SpawnEvent (.OutItem (Utilities|Array|Random (Variables|Default|GetEvents))))
    (else
      (Development|PrintText "No events initialized!"))))

(event Custom|SpawnSpecificEvent
  (params (EventClass :type BP%20Event%20Actor%20Class%20Reference))
  ;[0.15 0.15 0.15 0.5] SpawnSpecificEvent
  (bind _array_element (Utilities|Array|ForEachLoopwithBreak (Variables|Default|GetEvents))
    (:LoopBody
      (if (== (Utilities|GetClass _array_element) EventClass)
        (Default|SpawnEvent _array_element)
        (Development|PrintText (Utilities|Text|FormatText "ForceSpawned {name}" _array_element))))))

(event EventBeginPlay
  ;[0.15 0.15 0.15 0.5] Setup All Event spawners
  (for _array_element (Variables|Default|GetEvents)
    (Default|InitEvent _array_element)
    (Development|PrintText (Utilities|Text|FormatText "Setup the {x} event spawner" (Utilities|GetObjectName _array_element))))
  (Development|PrintText "Finished initializing all events")
  ;[0.15 0.15 0.15 0.5] Call for one of the event spawners to do their thing (I:E, spawn an event)
  (bind _asdata_jeu_du_bidou (Utilities|Casting|CastToDataJeuDuBidou (Game|GetGameInstance)))
  (Variables|Default|SetAs%20Data%20Jeu%20Du%20Bidou _asdata_jeu_du_bidou)
  (Variables|/Game/_Project/Data/DataJeuDuBidou.DataJeuDuBidou_C|SetEventManager _asdata_jeu_du_bidou self)
  (EventDispatchers|BindEventtoCallRandomEvent _asdata_jeu_du_bidou (delegate Custom|TrySpawnEvent)))

(fn ConstructionScript)
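; Event spawner that initializes, triggers and stops a pool of event entities.
; Init uses entities already listed in the active list or creates them up to a maximum, then saves the list.
; Spawn derives a clamped count from GameInstance difficulty, then starts or repositions randomly drawn entities, shrinking the working list and restoring it afterwards.
; Stop signals the event's end and force-stops every active entity.
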(event EventSpawnEvent
  ;[0.15 0.15 0.15 0.5] Spawn X events
  (bind _numtospawn (CallFunction|GetNumEntitytoSpawn))
  (Utilities|FlowControl|ForLoopwithBreak 0 _numtospawn :!label _label
    (:LoopBody
      (Utilities|IsValid (.OutItem (Utilities|Array|Random (Variables|Default|GetCurrentActiveEntities)))
        (:Is%20Valid
          (if (Variables|Default|GetAreEventsAlreadySpawned)
            (Class|BPIEventHelperFuncs|StartEvent(Message) (.OutItem (Utilities|Array|Random (Variables|Default|GetCurrentActiveEntities))))
            (else
              (CallFunction|MoveEventtoSpawnPoint (.OutItem (Utilities|Array|Random (Variables|Default|GetCurrentActiveEntities))))))
          (Rendering|SetActorHiddenInGame (.OutItem (Utilities|Array|Random (Variables|Default|GetCurrentActiveEntities))) false)
          (Utilities|Array|AddUnique (Variables|Default|GetCheckedListEntities) (.OutItem (Utilities|Array|Random (Variables|Default|GetCurrentActiveEntities))))
          (Utilities|Array|RemoveItem (Variables|Default|GetCurrentActiveEntities) (.OutItem (Utilities|Array|Random (Variables|Default|GetCurrentActiveEntities))))
          (if (Utilities|Array|IsEmpty (Variables|Default|GetCurrentActiveEntities))
            (goto _label Break)))))
    (:Completed
      (CallFunction|DebugTest (Utilities|Text|FormatText "Spawnign {x} of entity <= " _numtospawn))
      (Variables|Default|SetCurrentActiveEntities (Variables|Default|GetSavedListEntities))
      (Utilities|Array|Clear (Variables|Default|GetCheckedListEntities)))))

(event EventStopEvent
  ;[0.15 0.15 0.15 0.5] Stop all events
  (CallFunction|DebugTest "Stopping")
  (Default|CallEventStopped self)
  (for _array_element (Variables|Default|GetCurrentActiveEntities)
    (CallFunction|ForceStopEvent _array_element)))

(event EventInitEvent
  ;[0.15 0.15 0.15 0.5] Init Events
  (if (Variables|Default|GetAreEventsAlreadySpawned)
    (if (Utilities|Array|IsEmpty (Variables|Default|GetCurrentActiveEntities))
      (Development|PrintText "No events setup,  please add them in editor if they are already in scene")
      (else
        (for _array_element (Variables|Default|GetCurrentActiveEntities)
          (Class|BPIEventHelperFuncs|InitEvent(Message) _array_element))
        (Development|PrintText "Finished Initializing" :!label _label)
        (Variables|Default|SetSavedListEntities (Variables|Default|GetCurrentActiveEntities))))
    (else
      (CallFunction|DebugTest "Initializing ")
      (for _index (range 0 (Variables|Default|GetMaxNumEntities))
        (bind _eventcreated (CallFunction|InitEventSinglePoint))
        (Class|BPIEventHelperFuncs|InitEvent(Message) _eventcreated)
        (Utilities|Array|AddUnique (Variables|Default|GetCurrentActiveEntities) _eventcreated))
      (goto _label))))

(fn ConstructionScript
  (|CallParentFunction))

(fn GetNumEntitytoSpawn
  (bind _asdata_jeu_du_bidou (Utilities|Casting|CastToDataJeuDuBidou (Game|GetGameInstance)))
  (return (Math|Float|Truncate (Math|Float|Clamp(Float) (Math|Float|Lerp 1.0 (Math|Conversions|ToFloat(Integer) (Variables|Default|GetEntityMaxRandSpawn)) (Variables|/Game/_Project/Data/DataJeuDuBidou.DataJeuDuBidou_C|GetCurrentDifficultyVal _asdata_jeu_du_bidou)) 1.0 (Math|Conversions|ToFloat(Integer) (- (Variables|Default|GetMaxNumEntities) (Utilities|Array|Length (Variables|Default|GetCurrentActiveEntities))))))))
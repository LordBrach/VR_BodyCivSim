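; BP_TVEvent is a game event that switches an attached TV off when it spawns and back on when it initializes or stops.
; Each switch updates the TV state on the DataJeuDuBidou game instance, calls the TV's on or off event, and drives a spatialized cue and looping sound through BPCSoundPlayer.
; On BeginPlay it caches the game instance, then destroys itself if no TV is assigned.
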(event Custom|TurnOnTV
  ;[0.15 0.15 0.15 0.5] TurnOn TV
  (Default|SwitchTV (Variables|Default|GetAs%20Data%20Jeu%20Du%20Bidou) "NewEnumerator2")
  (Default|CETvon (Variables|Default|GetTV))
  (Default|PlaySoundSpatialized (Variables|Default|GetBPC_SoundPlayer) "TurnTVOn")
  (Default|StartLoopSound (Variables|Default|GetBPC_SoundPlayer) "TVOn"))

(event Custom|TurnOffTv
  (Default|SwitchTV (Variables|Default|GetAs%20Data%20Jeu%20Du%20Bidou) "NewEnumerator3")
  (Default|CETvOff (Variables|Default|GetTV))
  (Default|PlaySoundSpatialized (Variables|Default|GetBPC_SoundPlayer) "TVOff")
  (Default|StopLoopSound (Variables|Default|GetBPC_SoundPlayer) "TVOn"))

(event EventSpawnEvent
  (CallFunction|TurnOffTv))

(event EventStopEvent
  (CallFunction|TurnonTV))

(event EventInitEvent
  (CallFunction|TurnonTV))

(event EventBeginPlay
  ;[0.15 0.15 0.15 0.5] Setup
  (bind _asdata_jeu_du_bidou (Utilities|Casting|CastToDataJeuDuBidou (Game|GetGameInstance)))
  (Variables|Default|SetAs%20Data%20Jeu%20Du%20Bidou _asdata_jeu_du_bidou)
  (Utilities|IsValid (Variables|Default|GetTV)
    (:Is%20Not%20Valid
      (Development|PrintString "No tv attached to event" true true "(R=1.000000,G=0.000000,B=0.045802,A=1.000000)")
      (Actor|DestroyActor))))

(fn ConstructionScript
  (|CallParentFunction))
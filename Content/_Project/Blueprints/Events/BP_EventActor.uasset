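; Event actor, apparently a base, with init, spawn and stop events that print debug text, track a playing flag and fire an EventStopped dispatcher on stop.
; Helpers pre-spawn a hidden entity at an out-of-bounds point, then teleport it to the spawn point and send it a start message.
; Force-stop messages entities implementing BPI_EventHelperFuncs and hides this actor, otherwise destroys the entity.
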(event Custom|StopEvent
  (CallFunction|DebugTest "Stopping")
  (Variables|Default|SetIsPlaying false)
  (Default|CallEventStopped self))

(event Custom|SpawnEvent
  (CallFunction|DebugTest "Spawning")
  (Variables|Default|SetIsPlaying true))

(event Custom|InitEvent
  (CallFunction|DebugTest "Initializing "))

(event EventBeginPlay)

(event Collision|EventActorBeginOverlap
  (params (OtherActor :type Actor%20Object%20Reference)))

(event EventTick
  (params (DeltaSeconds :type Float%20%28single-precision%29)))

(fn ConstructionScript)

(fn DebugTest
  (params (IntroWord :type Text))
  (Development|PrintText (Utilities|Text|FormatText "{IntroWord} {event}" IntroWord (Utilities|GetObjectName self))))

(fn InitEventSinglePoint
  (bind _returnvalue (Game|SpawnActorfromClass (Variables|Default|GetEntityClassRef) (Transformation|GetRelativeTransform (Variables|Default|GetInitPoint%20%28Out%20of%20bounds%29)) "Undefined" "MultiplyWithRoot" 0 0))
  (Rendering|SetActorHiddenInGame _returnvalue true)
  (return _returnvalue))

(fn MoveEventtoSpawnPoint
  (params (Event :type Actor%20Object%20Reference))
  (Transformation|SetActorTransform Event (Transformation|GetWorldTransform (Variables|Default|GetSpawnPoint)) false true)
  (Class|BPIEventHelperFuncs|StartEvent(Message) Event)
  (return))

(fn ForceStopEvent
  (params (Event :type Actor%20Object%20Reference))
  (CallFunction|DebugTest "Stopping")
  (if (Utilities|DoesObjectImplementInterface Event "/Game/_Project/Blueprints/Events/BPI_EventHelperFuncs.BPI_EventHelperFuncs_C")
    (Class|BPIEventHelperFuncs|ForceStop(Message) Event)
    (Rendering|SetActorHiddenInGame true)
    (else
      (Actor|DestroyActor Event)))
  (return))
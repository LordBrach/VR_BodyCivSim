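; Event spawner that manages a single active event entity, with init, spawn and stop events.
; Init uses a pre-placed entity or creates one at a single point, then sends it an init message.
; Spawning starts or moves a hidden entity to its spawn point, while a visible one receives a spawn-while-playing message.
; Stopping force-stops entities implementing BPI_EventHelperFuncs, destroys others, and clears the reference.
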(event EventInitEvent
  ;[0.15 0.15 0.15 0.5] Init the event
  (CallFunction|DebugTest "Initializing ")
  (if (Variables|Default|GetAreEventsAlreadySpawned)
    (bind _currentactiveentity (Variables|Default|GetCurrentActiveEntity)
      (:then
        (Class|BPIEventHelperFuncs|InitEvent(Message) _currentactiveentity))
      (:else
        (Development|PrintText "No events setup,  please add them in editor if they are already in scene")))
    (else
      (bind _eventcreated (CallFunction|InitEventSinglePoint))
      (bind _output_get (Variables|Default|SetCurrentActiveEntity _eventcreated))
      (Class|BPIEventHelperFuncs|InitEvent(Message) _output_get))))

(event EventSpawnEvent
  (bind _currentactiveentity (Variables|Default|GetCurrentActiveEntity))
  ;[0.15 0.15 0.15 0.5] Spawn the event
  (if (Variables|/Script/Engine.Actor|GetbHidden (Variables|Default|GetCurrentActiveEntity))
    (if (Variables|Default|GetAreEventsAlreadySpawned)
      (Class|BPIEventHelperFuncs|StartEvent(Message) _currentactiveentity)
      (else
        (CallFunction|MoveEventtoSpawnPoint _currentactiveentity)))
    (Variables|Default|SetIsPlaying true)
    (Rendering|SetActorHiddenInGame false)
    (else
      (CallFunction|DebugTest "Spawning")
      (Class|BPIEventHelperFuncs|SpawnWhileEventPlaying(Message) (Variables|Default|GetCurrentActiveEntity)))))

(event EventStopEvent
  ;[0.15 0.15 0.15 0.5] Stop the event by force
  (bind _currentactiveentity (Variables|Default|GetCurrentActiveEntity)
    (:then
      (CallFunction|DebugTest "Stopping")
      (if (Utilities|DoesObjectImplementInterface _currentactiveentity "/Game/_Project/Blueprints/Events/BPI_EventHelperFuncs.BPI_EventHelperFuncs_C")
        (Class|BPIEventHelperFuncs|ForceStop(Message) (Variables|Default|GetCurrentActiveEntity))
        (else
          (Actor|DestroyActor (Variables|Default|GetCurrentActiveEntity))))
      (Variables|Default|SetCurrentActiveEntity 0)
      (Variables|Default|SetIsPlaying false))
    (:else)))

(fn ConstructionScript
  (|CallParentFunction))